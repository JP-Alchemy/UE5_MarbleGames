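; BP_WinVolume is a trigger volume that advances the game to the next level when the player overlaps it.
; As wired, it calls CompleteLevel only while BP_Gem actors still exist, since IsCrystalRemaining is not negated.
; CompleteLevel finds the current level in the LevelNames array and opens the following entry by name, doing nothing on the last level.
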(event Collision|EventActorBeginOverlap
  (params (OtherActor :type Actor%20Object%20Reference))
  (Utilities|MIsPlayer OtherActor
    (:IsPlayer
      (if (CallFunction|IsCrystalRemaining)
        (CallFunction|CompleteLevel)))))

(fn ConstructionScript)

(fn IsCrystalRemaining
  (bind _outactors (Actor|GetAllActorsOfClass "/Game/Blueprints/Actors/BP_Gem.BP_Gem_C"))
  (return (> (Utilities|Array|Length _outactors) 0)))

(fn CompleteLevel
  (if (not (CallFunction|IsLastLevel))
    (CallFunction|LoadNextLevel)))

(fn IsLastLevel
  (return (== (Utilities|Array|LastIndex (Variables|Default|GetLevelNames)) (CallFunction|GetCurrentLevelIndex))))

(fn GetCurrentLevelIndex
  (bind _returnvalue (Game|GetCurrentLevelName true))
  (return (Utilities|Array|FindItem (Variables|Default|GetLevelNames) (Utilities|String|StringToName _returnvalue))))

(fn LoadNextLevel
  (Game|OpenLevel(byName) (CallFunction|GetNextLevelName)))

(fn GetNextLevelName
  (return (Utilities|Array|Get(acopy) (Variables|Default|GetLevelNames) (+ (CallFunction|GetCurrentLevelIndex) 1))))