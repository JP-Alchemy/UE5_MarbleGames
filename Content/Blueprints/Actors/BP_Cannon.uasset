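; BP_Cannon is an actor that automatically fires projectiles in a repeating cycle from BeginPlay.
; After a configurable delay, it spawns a BP_Projectile at the Arrow component's location and rotation, using a configurable uniform scale.
; A timeline then drives the Cannon component's recoil along local Y, and its Cannon Fired event track loops execution back to the delay.
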(event EventBeginPlay
  (Utilities|FlowControl|Delay (Variables|Projectile|GetProjectileDelay) :!label _label)
  (CallFunction|SpawnProjectile)
  (bind _recoil (Timeline|CannonAnimation PlayFromStart)
    (:Update
      (Transformation|SetRelativeLocation (Variables|Default|GetCannon) (Math|Vector|MakeVector 0.0 _recoil 0.0) false false))
    (:CannonFired
      (goto _label))))

(event Collision|EventActorBeginOverlap
  (params (OtherActor :type Actor%20Object%20Reference)))

(event EventTick
  (params (DeltaSeconds :type Float%20%28single-precision%29)))

(fn ConstructionScript)

(fn SpawnProjectile
  (bind _arrow (Variables|Default|GetArrow))
  (Game|SpawnActorfromClass "/Game/Blueprints/Actors/BP_Projectile.BP_Projectile_C" (Math|Transform|MakeTransform (Transformation|GetWorldLocation _arrow) (Transformation|GetWorldRotation _arrow) (Math|Conversions|ToVector(Float) (Variables|Projectile|GetProjectileScale))) "Undefined" 0 0))