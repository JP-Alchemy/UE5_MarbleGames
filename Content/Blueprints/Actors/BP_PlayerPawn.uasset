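; BP_PlayerPawn is a player pawn that rolls a physics sphere and restarts the level when it takes any damage.
; Forward/back and left/right axis inputs share one torque call on the sphere, scaled by an acceleration multiplier.
; The camera fades in on BeginPlay, while the Restart Level macro fades out, waits for the fade, then reopens the current level by name.
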(event EventBeginPlay
  (CameraFades|StartCameraFade :self (Game|GetPlayerCameraManager 0) :FromAlpha 1.0 :Duration 2.0))

(event Collision|EventActorBeginOverlap
  (params (OtherActor :type Actor%20Object%20Reference)))

(event EventTick
  (params (DeltaSeconds :type Float%20%28single-precision%29)))

(event Game|Damage|EventAnyDamage
  (params (Damage :type Float%20%28single-precision%29) (DamageType :type Damage%20Type%20Object%20Reference) (InstigatedBy :type Controller%20Object%20Reference) (DamageCauser :type Actor%20Object%20Reference))
  (Utilities|RestartLevel))

(event Input|AxisEvents|InputAxisForward_Backward
  (params (AxisValue :type Float%20%28single-precision%29))
  (bind _accelmultiplier (Variables|Default|GetAccelMultiplier))
  (Class|PrimitiveComponent|AddTorqueinRadians (Variables|Default|GetSphere) (Math|Vector|MakeVector (* (stale Input|AxisEvents|InputAxisLeft_Right AxisValue) _accelmultiplier) (* AxisValue _accelmultiplier) 0.0) "None" true))

(event Input|AxisEvents|InputAxisLeft_Right
  (params (AxisValue :type Float%20%28single-precision%29))
  (bind _accelmultiplier (Variables|Default|GetAccelMultiplier))
  (Class|PrimitiveComponent|AddTorqueinRadians (Variables|Default|GetSphere) (Math|Vector|MakeVector (* AxisValue _accelmultiplier) (* (stale Input|AxisEvents|InputAxisForward_Backward AxisValue) _accelmultiplier) 0.0) "None" true))

(fn ConstructionScript)