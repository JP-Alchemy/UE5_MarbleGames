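; BP_Gem is a gem actor that flies into the player and vanishes when touched.
; A sphere overlap passes through an Is Player macro check against player pawn 0, then plays CollisionTimeline.
; Timeline tracks feed AnimateDestroy, which lerps location toward the player and scale and point light intensity toward zero, each from its current value.
; The actor destroys itself when the timeline finishes.
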(event OnComponentBeginOverlap(Sphere)
  (params (OverlappedComponent :type Primitive%20Component%20Object%20Reference) (OtherActor :type Actor%20Object%20Reference) (OtherComp :type Primitive%20Component%20Object%20Reference) (OtherBodyIndex :type Integer) (bFromSweep :type Boolean) (SweepResult :type Hit%20Result%20Structure%20%28by%20ref%29))
  (Utilities|MIsPlayer OtherActor
    (:IsPlayer
      (bind (_direction _scale _intensity _location) (Timeline|CollisionTimeline Play)
        (:Update
          (CallFunction|AnimateDestroy _scale _intensity _location))
        (:Finished
          (Actor|DestroyActor))))))

(event EventBeginPlay)

(event Collision|EventActorBeginOverlap
  (params (OtherActor :type Actor%20Object%20Reference)))

(event EventTick
  (params (DeltaSeconds :type Float%20%28single-precision%29)))

(fn ConstructionScript)

(fn SetLocation
  (params (Alpha :type Float%20%28single-precision%29))
  (Transformation|SetActorLocation (Math|Vector|Lerp(Vector) (Transformation|GetActorLocation) (Transformation|GetActorLocation (Game|Player|GetPlayerPawn 0)) Alpha) false false))

(fn SetScale
  (params (Alpha :type Float%20%28single-precision%29))
  (Transformation|SetActorScale3D (Math|Vector|Lerp(Vector) (Transformation|GetActorScale3D) "0, 0, 0" Alpha)))

(fn SetIntensity
  (params (Alpha :type Float%20%28double-precision%29))
  (bind _pointlight (Variables|Default|GetPointLight))
  (Rendering|Components|Light|SetIntensity _pointlight (Math|Float|Lerp (Variables|/Script/Engine.LightComponentBase|GetIntensity _pointlight) 0.0 Alpha)))

(fn AnimateDestroy
  (params (Scale :type Float%20%28single-precision%29) (Intensity :type Float%20%28double-precision%29) (Location :type Float%20%28single-precision%29))
  (CallFunction|SetLocation Location)
  (CallFunction|SetScale Scale)
  (CallFunction|SetIntensity Intensity))